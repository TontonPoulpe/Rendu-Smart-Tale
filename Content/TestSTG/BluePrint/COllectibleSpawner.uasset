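; Collectible spawner actor that scatters health-losing and health-gaining fruit pickups at random positions around itself.
; A Delay on Tick throttles spawning to roughly one attempt per second.
; Each attempt randomly spawns FruitLoseHP, FruitWinHP or nothing, using a three-way switch.
; The spawn point is the actor's location plus a random offset on all three axes, with its upper bound set by MaxPos.
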(event EventBeginPlay)

(event EventTick
  (params (DeltaSeconds :type Float%20%28single-precision%29))
  (bind _maxpos (Variables|Default|GetMaxPos))
  ;[1 1 1] Spawn des objets en random
  (Utilities|FlowControl|Delay 1.0)
  (Variables|Default|SetSpawnRang (Math|Random|RandomIntegerinRange 0 2))
  (Variables|Default|SetNewPosition (Math|Vector|MakeVector (Math|Random|RandomFloatinRange -5e+02 _maxpos) (Math|Random|RandomFloatinRange -5e+02 _maxpos) (Math|Random|RandomFloatinRange -5e+02 _maxpos)))
  (switch int (Variables|Default|GetSpawnRang)
    (:0
      (Game|SpawnActorfromClass "/Game/TestSTG/Prefab/InteractionLife/FruitLoseHP.FruitLoseHP_C" (Math|Transform|MakeTransform (+ (Variables|Default|GetNewPosition) (Transformation|GetActorLocation self)) "0, 0, 0" "1,1,1") "Undefined" 0 0))
    (:1
      (Game|SpawnActorfromClass "/Game/TestSTG/Prefab/InteractionLife/FruitWinHP.FruitWinHP_C" (Math|Transform|MakeTransform (+ (Variables|Default|GetNewPosition) (Transformation|GetActorLocation self)) "0, 0, 0" "1,1,1") "Undefined" 0 0))))

(fn ConstructionScript)